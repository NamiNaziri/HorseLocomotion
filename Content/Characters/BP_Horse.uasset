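; Player-controlled horse character with a mounted rider who toggles drawing and stowing a bow on the F key, using montage notifies to reattach it.
; Camera-relative move input is smoothly interpolated into a steering direction that drives movement.
; Tick turns the body toward the last significant velocity at a curve-driven rate based on angular difference, records HeadingYaw, and draws movement debug.
; Construction makes tack, armour, mane and wing meshes follow the horse's pose.
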(event Input|EnhancedActionEvents|EnhancedInputActionIA_MouseLook
  (params (ActionValue :type Vector%202D%20Structure) (ElapsedSeconds :type Float%20%28double-precision%29) (TriggeredSeconds :type Float%20%28double-precision%29) (InputAction :type Input%20Action%20Object%20Reference :default "/Game/Input/Actions/IA_MouseLook.IA_MouseLook"))
  (bind (_x _y) (Math|Vector2D|BreakVector2D ActionValue))
  (Pawn|Input|AddControllerPitchInput _y)
  (Pawn|Input|AddControllerYawInput _x))

(event Input|EnhancedActionEvents|EnhancedInputActionIA_Move
  (params (ActionValue :type Vector%202D%20Structure) (ElapsedSeconds :type Float%20%28double-precision%29) (TriggeredSeconds :type Float%20%28double-precision%29) (InputAction :type Input%20Action%20Object%20Reference :default "/Game/Input/Actions/IA_Move.IA_Move"))
  (bind (_x _y) (Math|Vector2D|BreakVector2D ActionValue))
  (bind _returnvalue (Game|GetPlayerCameraManager 0))
  (bind _returnvalue_2 (Utilities|Time|GetWorldDeltaSeconds))
  (bind _returnvalue_3 (Camera|GetCameraRotation _returnvalue))
  (bind _returnvalue_4 (Math|Rotator|GetRotationXVector _returnvalue_3))
  (bind _returnvalue_5 (Math|Vector|GetRightVector _returnvalue_3))
  (bind _returnvalue_6 (* _y _returnvalue_4))
  (bind _returnvalue_7 (* _x _returnvalue_5 1.0))
  (bind _returnvalue_8 (+ _returnvalue_6 _returnvalue_7))
  (bind _returnvalue_9 (Math|Vector|Normalize _returnvalue_8))
  (Variables|Default|SetAcceleration (Math|Interpolation|VInterpTo (Variables|Default|GetAcceleration) _returnvalue_9 _returnvalue_2 8.0))
  (bind _output_get (Variables|Default|SetAccelerationRot (Math|Interpolation|RInterpTo (Variables|Default|GetAccelerationRot) (Math|Conversions|RotationFromXVector _returnvalue_9) _returnvalue_2 3.0)))
  (Pawn|Input|AddMovementInput (Math|Rotator|GetRotationXVector _output_get) 1.0 false)
  (Class|PoseSearchLibraryExtended|DrawPredictedTrajectory self ActionValue 1.0))

(event EventBeginPlay
  (bind _returnvalue (Game|GetPlayerController 0))
  (bind _charactermovement (Variables|Character|GetCharacterMovement))
  (bind _returnvalue_2 (PlayerController|LocalPlayerSubsystems|GetEnhancedInputLocalPlayerSubsystem _returnvalue))
  (Transformation|AttachComponentToComponent (Variables|Default|GetBow) (Variables|Default|GetRider) "attach_back" "SnapToTarget" "SnapToTarget" "SnapToTarget" true)
  (Input|AddMappingContext _returnvalue_2 "/Game/Input/IMC_Default.IMC_Default" 0 "(bIgnoreAllPressedKeysUntilRelease=True,bForceImmediately=False,bNotifyUserSettings=False)")
  (Input|AddMappingContext _returnvalue_2 "/Game/Input/IMC_MouseLook.IMC_MouseLook" 0 "(bIgnoreAllPressedKeysUntilRelease=True,bForceImmediately=False,bNotifyUserSettings=False)")
  (Variables|/Script/Engine.CharacterMovementComponent|SetMaxWalkSpeed _charactermovement 309.0)
  (Variables|/Script/Engine.CharacterMovementComponent|SetMaxAcceleration _charactermovement 5.5e+02))

(event Collision|EventActorBeginOverlap
  (params (OtherActor :type Actor%20Object%20Reference)))

(event EventTick
  (params (DeltaSeconds :type Float%20%28single-precision%29))
  (bind _returnvalue (Transformation|GetActorLocation))
  (bind _returnvalue_2 (Transformation|GetActorRotation))
  (bind _returnvalue_3 (Transformation|GetActorLocation))
  (bind _returnvalue_4 (Transformation|GetActorLocation))
  (bind _charactermovement (Variables|Character|GetCharacterMovement))
  (bind _charactermovement_2 (Variables|Character|GetCharacterMovement))
  (bind _charactermovement_3 (Variables|Character|GetCharacterMovement))
  (bind _velocity (Variables|/Script/Engine.MovementComponent|GetVelocity _charactermovement_2))
  (Utilities|FlowControl|Sequence
    (:then_0
      (Rendering|Debug|DrawDebugArrow :LineStart _returnvalue_3 :LineEnd (+ _returnvalue_3 (* (Transformation|GetActorForwardVector) 255.0)) :ArrowSize 1.0)
      (if (>= (Math|Vector|VectorLengthXY (Variables|/Script/Engine.MovementComponent|GetVelocity _charactermovement)) 119.0)
        (Variables|/Script/Engine.CharacterMovementComponent|SetMaxAcceleration _charactermovement 7.5e+02)
        (Variables|/Script/Engine.CharacterMovementComponent|SetBrakingDecelerationWalking _charactermovement 1.0)
        (else
          (Variables|/Script/Engine.CharacterMovementComponent|SetMaxAcceleration _charactermovement 7.5e+02))))
    (:then_2
      (Rendering|Debug|DrawDebugString (Transformation|GetActorLocation) (Utilities|String|ToString(Text) (Utilities|Text|FormatText "Speed 2D: {A} 
Velocity: {B} 
Max Acceleration:{C} 
Breaking Decel: {d} 
Curr Acceleration:{E} 
" (Utilities|String|ToString(Float) (Math|Vector|VectorLengthXY (Variables|/Script/Engine.MovementComponent|GetVelocity (Variables|Character|GetCharacterMovement)))) (Utilities|String|ToString(Vector) (Variables|/Script/Engine.MovementComponent|GetVelocity (Variables|Character|GetCharacterMovement))) (Utilities|String|ToString(Float) (Class|CharacterMovementComponent|GetMaxAcceleration _charactermovement_3)) (Utilities|String|ToString(Float) (Class|CharacterMovementComponent|GetMaxBrakingDeceleration _charactermovement_3)) (Utilities|String|ToString(Vector) (Pawn|Components|CharacterMovement|GetCurrentAcceleration _charactermovement_3)))) 0 "(R=1.000000,G=1.000000,B=1.000000,A=1.000000)"))
    (:then_3
      (if (> (Math|Vector|VectorLengthXY _velocity) 2.0)
        (Variables|Default|SetCachedVelocity _velocity))
      (Variables|Default|SetHeadingYaw (.Yaw (Math|Rotator|BreakRotator (Math|Rotator|Delta(Rotator) (Math|Conversions|RotationFromXVector (Variables|Default|GetCachedVelocity)) _returnvalue_2))))
      (Transformation|SetActorRotation (Math|Interpolation|RInterpTo _returnvalue_2 (Math|Conversions|RotationFromXVector (Variables|Default|GetCachedVelocity)) DeltaSeconds (.OutValue (Class|AnimationWarpingLibrary|GetFloatValuefromCurve "/Game/Blueprints/Character/Movement/Curve_RotationInterpSpeed.Curve_RotationInterpSpeed" (Math|Float|Absolute(Float) (.Yaw (Math|Rotator|BreakRotator (Math|Rotator|Delta(Rotator) (Math|Conversions|RotationFromXVector (Variables|Default|GetCachedVelocity)) _returnvalue_2))))))))
      (Rendering|Debug|DrawDebugArrow _returnvalue_4 (+ _returnvalue_4 (* (Variables|Default|GetCachedVelocity) 255.0)) 1.0 "(R=0.029579,G=0.434050,B=1.000000,A=1.000000)" 0.0 0.0)
      (Development|PrintString (Utilities|String|ToString(Text) (Utilities|Text|FormatText "Delta: {A} 
Speed:{B}" (Math|Float|Absolute(Float) (.Yaw (Math|Rotator|BreakRotator (Math|Rotator|Delta(Rotator) (Math|Conversions|RotationFromXVector (Variables|Default|GetCachedVelocity)) _returnvalue_2)))) (.OutValue (Class|AnimationWarpingLibrary|GetFloatValuefromCurve "/Game/Blueprints/Character/Movement/Curve_RotationInterpSpeed.Curve_RotationInterpSpeed" (Math|Float|Absolute(Float) (.Yaw (Math|Rotator|BreakRotator (Math|Rotator|Delta(Rotator) (Math|Conversions|RotationFromXVector (Variables|Default|GetCachedVelocity)) _returnvalue_2)))))))) true true "(R=0.000000,G=0.660000,B=1.000000,A=1.000000)" 0.0)
      (Rendering|Debug|DrawDebugArrow _returnvalue (+ _returnvalue (* (Math|Vector|GetForwardVector (Variables|Default|GetAccelerationRot)) 255.0)) 1.0 "(R=1.000000,G=0.000000,B=0.018797,A=1.000000)" 0.0 0.0))))

(event Input|KeyboardEvents|DebugKeyF
  (params (Key :type Key%20Structure :default "None") (ActionValue :type Input%20Action%20Value%20Structure))
  (bind _rider (Variables|Default|GetRider))
  (:Pressed
    (Utilities|FlowControl|FlipFlop
      (:A
        (bind _notifyname (Animation|Montage|PlayMontage _rider "/Game/Animations/Rider/Bow/Draw_Back_L_Montage.Draw_Back_L_Montage")
          (:OnCompleted
            (Variables|Default|SetbHoldingBow true))
          (:OnNotifyBegin
            (if (== _notifyname "AttachToHand")
              (Transformation|AttachComponentToComponent (Variables|Default|GetBow) (Variables|Default|GetRider) "hand_lSocket" "SnapToTarget" "SnapToTarget" "SnapToTarget" true)))))
      (:B
        (bind _notifyname_2 (Animation|Montage|PlayMontage _rider "/Game/Animations/Rider/Bow/Store_Back_L_Montage.Store_Back_L_Montage")
          (:then
            (Variables|Default|SetbHoldingBow false))
          (:OnNotifyBegin
            (if (== _notifyname_2 "AttachToBack")
              (Transformation|AttachComponentToComponent (Variables|Default|GetBow) (Variables|Default|GetRider) "attach_back" "SnapToTarget" "SnapToTarget" "SnapToTarget" true))))))))

(fn ConstructionScript
  (Components|SkinnedMesh|SetLeaderPoseComponent (Variables|Default|GetReins) (Variables|Character|GetMesh) false false))